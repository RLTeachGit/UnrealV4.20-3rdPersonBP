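; Door frame Blueprint with a combination lock that opens its door when pads are stepped on in the PadSequence order.
; DoStepOnPad compares each pad to the expected step, advancing on a match and resetting on a mistake or after unlocking.
; Hitting the first pad always restarts the sequence.
; Completing it plays a Timeline that smoothly yaws the door relative to the frame up to MaxOpen.
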(event Collision|EventActorBeginOverlap
  (params (OtherActor :type Actor%20Object%20Reference)))

(event EventTick
  (params (DeltaSeconds :type Float%20%28single-precision%29)))

(event Custom|DoStepOnPad
  (params (Pad :type Pad%20BP%20Object%20Reference))
  ;[1 1 1] Always reset if first pad hit, this allows player to easly start again
  (CallFunction|FirstPadReset Pad)
  (bind _iscorrect (CallFunction|IsCorrectPad Pad))
  (if _iscorrect
    (bind _isfinished (CallFunction|DoNextUnlock))
    ;[1 1 1] If at the end of the sequence we unlock the door, if not we dont need to do anything, as next index already set
    (if _isfinished
      (CallFunction|DoDoorOpen)
      (CallFunction|ResetLock :!label _label))
    (else
      (goto _label))))

(event Custom|DoDoorOpen
  ;[1 1 1] Smoothly go from 0-1 over 1 second
  (bind _openfraction (Timeline|Timeline_0 PlayFromStart)
    (:Update
      ;[1 1 1] Set Doors rotation relative to parent (DoorFrame)
      (Transformation|SetRelativeRotation (Variables|Default|GetDoor) (Math|Rotator|MakeRotator 0.0 0.0 (* _openfraction (Variables|Default|GetMaxOpen))) false false))
    (:Finished
      ;[1 1 1] Needed as you can't connect node execute exit to entry on same node
      (CallFunction|DoNothing)
      (Timeline|Timeline_0 SetNewTime))))

(fn ConstructionScript)

(fn DoNothing
  ;[1 1 1] Allows you to connect execution exit of node to its own execution entry
)

(fn IsCorrectPad
  (params (Pad :type Pad%20BP%20Object%20Reference))
  ;[1 1 1] Validate if input pad is the one we are expecting
  (return (== Pad (Utilities|Array|Get(acopy) (Variables|Default|GetPadSequence) (Variables|Default|GetCurrentStep)))))

(fn DoNextUnlock
  ;[1 1 1] Increment unlock index, if at end of array, we are finished so unlock
  (bind _result (Math|Integer|IncrementInt (Variables|Default|GetCurrentStep))
    (:%20%20
      (return (== _result (Utilities|Array|Length (Variables|Default|GetPadSequence)))))))

(fn ResetLock
  ;[1 1 1] Set Index to zero to reset lock
  (Variables|Default|SetCurrentStep 0))

(fn DebugStep
  (params (Pad :type Pad%20BP%20Object%20Reference))
  (bind _currentstep (Variables|Default|GetCurrentStep))
  ;[1 1 1] Display Debug info for door
  (Development|PrintText (Utilities|Text|FormatText "Stepped on ({Step}) Index {Index} Expected {Expected}" (Utilities|Text|ToText(String) (Utilities|GetObjectName Pad)) _currentstep (Utilities|Text|ToText(String) (Utilities|GetObjectName (Utilities|Array|Get(acopy) (Variables|Default|GetPadSequence) _currentstep))))))

(fn FirstPadReset
  (params (Pad :type Pad%20BP%20Object%20Reference))
  ;[1 1 1] Also reset lock if first Pad Hit
  (if (== (Utilities|Array|Get(acopy) (Variables|Default|GetPadSequence)) Pad)
    (CallFunction|ResetLock)))